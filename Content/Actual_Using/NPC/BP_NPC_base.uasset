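; Base NPC character Blueprint with damage reactions, a melee-style attack trace, nav link jumping and ragdoll death.
; Damage feeds the health bar component and picks a punch or neck-break montage by amount; neck-break deaths wait before ragdolling, then the actor is destroyed on a timer.
; Sphere overlap toggles the Attack component's visibility, while AttackFun delegates hit tracing to the health component.
; Nav link jumps use LaunchCharacter with velocity computed toward the destination.
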(event SignalPlayerDeath(HealthBar_Component)
  (if (Variables|Default|GetIsTakedown)
    _
    (else
      (Utilities|FlowControl|Delay 2.6)))
  (CallFunction|TriggerDeath))

(event OnComponentBeginOverlap(Sphere)
  (params (OverlappedComponent :type Primitive%20Component%20Object%20Reference) (OtherActor :type Actor%20Object%20Reference) (OtherComp :type Primitive%20Component%20Object%20Reference) (OtherBodyIndex :type Integer) (bFromSweep :type Boolean) (SweepResult :type Hit%20Result%20Structure%20%28by%20ref%29))
  (Rendering|SetVisibility (Variables|Default|GetAttack) true false))

(event OnComponentEndOverlap(Sphere)
  (params (OverlappedComponent :type Primitive%20Component%20Object%20Reference) (OtherActor :type Actor%20Object%20Reference) (OtherComp :type Primitive%20Component%20Object%20Reference) (OtherBodyIndex :type Integer))
  (Rendering|SetVisibility (Variables|Default|GetAttack) false false))

(event Collision|EventActorBeginOverlap
  (params (OtherActor :type Actor%20Object%20Reference)))

(event Game|Damage|EventAnyDamage
  (params (Damage :type Float%20%28single-precision%29) (DamageType :type Damage%20Type%20Object%20Reference) (InstigatedBy :type Controller%20Object%20Reference) (DamageCauser :type Actor%20Object%20Reference))
  (bind _healthbar_component (Variables|Default|GetHealthBar_Component))
  (bind _output_get (Variables|Default|SetIsTakedown (<= Damage 2e+01)))
  (if _output_get
    (Default|ProcessDamage _healthbar_component Damage)
    (Animation|PlayAnimMontage "/Game/Actual_Using/NPC/Animations/Attacks/AM_Hit_punch.AM_Hit_punch" 1.0 "None")
    (else
      (Default|ProcessDamage _healthbar_component Damage)
      (Animation|PlayAnimMontage "/Game/Actual_Using/NPC/Animations/Attacks/AM_Hit_Breakneck.AM_Hit_Breakneck" 1.0 "None"))))

(event EventNavLinkinRange
  (params (Agent :type Actor%20Object%20Reference) (NavLinkDestination :type Vector :default "0, 0, 0"))
  (bind (_x _y _z) (Class|KismetMathLibrary|BreakVector3f NavLinkDestination))
  (bind _returnvalue (Transformation|GetActorLocation))
  (bind (_x_2 _y_2 _z_2) (Class|KismetMathLibrary|BreakVector3f _returnvalue))
  (Character|LaunchCharacter (Math|Vector|MakeVector (|((destinationX-StartX)/{FDC75289-4CAE-65AC-8B24-AC8C242A011A}) _x _x_2) (|((destinationY-StartY)/{FDC75289-4CAE-65AC-8B24-AC8C242A011A}) _y _y_2) (|((destinationHeight-(StartHeight-(((Power({FDC75289-4CAE-65AC-8B24-AC8C242A011A},2))*0.500000)*{CA7CF131-4971-20B4-4B54-1BAA2A3BC89C})))/{FDC75289-4CAE-65AC-8B24-AC8C242A011A}) _z _z_2)) true true))

(fn ConstructionScript)

(fn TriggerDeath
  (Physics|SetSimulatePhysics (Variables|Character|GetMesh) true)
  (Pawn|Components|CharacterMovement|DisableMovement (Variables|Character|GetCharacterMovement))
  (Utilities|Time|SetTimerbyFunctionName 0 "FinalizeDeath" 3.0))

(fn FinalizeDeath
  (Actor|DestroyActor))

(fn AttackFun
  (Default|TrytoHit (Variables|Default|GetHealthBar_Component) (Variables|Default|GetLienTraceStart) (Variables|Default|GetLineTraceEnd)))