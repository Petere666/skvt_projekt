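; BP_EMP_Button is a pushable button actor for the EMP box that animates its press when EMP_Button_Event is called.
; A timeline lerps the button model's relative location from start to pushed, then plays in reverse after a delay to release it.
; A DoOnce gate blocks repeat presses and resets shortly after the release begins.
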(event Custom|EMP_Button_Event
  ;[1 1 1] button pushed animation
  (Utilities|FlowControl|Sequence
    (:then_0
      (Utilities|FlowControl|DoOnce false :!label _label
        (:Completed
          (Utilities|FlowControl|Sequence
            (:then_0
              (bind _buttom_track (Timeline|EMP_button_timeline PlayFromStart)
                (:Update
                  (Transformation|SetRelativeLocation (Variables|Default|GetEMP_ButtonModel) (Math|Vector|Lerp(Vector) (Variables|Default|Getstart) (Variables|Default|Getpushed) _buttom_track) false false))))
            (:then_1
              (Utilities|FlowControl|Delay 5.5)
              (Timeline|EMP_button_timeline ReverseFromEnd))))))
    (:then_1
      (Utilities|FlowControl|Delay 6.0)
      (goto _label Reset))))

(event EventBeginPlay)

(event Collision|EventActorBeginOverlap
  (params (OtherActor :type Actor%20Object%20Reference)))

(event EventTick
  (params (DeltaSeconds :type Float%20%28single-precision%29)))

(fn ConstructionScript)