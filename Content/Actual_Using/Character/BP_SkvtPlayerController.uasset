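; BP_SkvtPlayerController is a player controller that sets up Enhanced Input and owns the player's HUD.
; On BeginPlay, if the input subsystem is valid, it adds IMC_Default, makes a second mapping-context call with no context set, then creates WBP_PlayerHUD and adds it to the viewport.
; UpdateHealthBar forwards the passed component to the stored HUD widget when it is valid.
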(event EventBeginPlay
  (bind _self self)
  (bind _returnvalue (PlayerController|LocalPlayerSubsystems|GetEnhancedInputLocalPlayerSubsystem _self))
  (Utilities|IsValid _returnvalue
    (:Is%20Valid
      (Input|AddMappingContext _returnvalue "/Game/Actual_Using/Character/Input/IMC_Default.IMC_Default" 0 "(bIgnoreAllPressedKeysUntilRelease=True,bForceImmediately=False)")
      (Input|AddMappingContext _returnvalue 0 0 "(bIgnoreAllPressedKeysUntilRelease=True,bForceImmediately=False)")
      (CallFunction|CreatePlayerHUD))))

(fn ConstructionScript)

(fn CreatePlayerHUD
  (bind _returnvalue (UserInterface|CreateWidget "/Game/Actual_Using/UI/Widgets/WBP_PlayerHUD.WBP_PlayerHUD_C" self))
  (bind _output_get (Variables|Default|SetHUDWidget _returnvalue))
  (UserInterface|Viewport|AddtoViewport _output_get 0))

(fn UpdateHealthBar
  (params (NewComponent :type Health%20Bar%20Component%20Object%20Reference))
  (bind _hudwidget (Variables|Default|GetHUDWidget))
  (Utilities|IsValid _hudwidget
    (:Is%20Valid
      (Default|UpdateHealthBar _hudwidget NewComponent))))